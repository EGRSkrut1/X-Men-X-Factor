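; BP_AbilityComponent is a bare ability component for characters that tracks whether an ability is running.
; StartAbility and StopAbility set and clear the IsRunning flag, and CanStart refuses a start while it is set.
; GetOwningComponent casts an outer object to BP_AbilityComponent and returns it if valid.
; InitAbility is an empty stub, and the event graph has no active logic.
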(event EventBeginPlay)

(event EventTick
  (params (DeltaSeconds :type Float%20%28single-precision%29)))

(fn StartAbility
  (Variables|Default|SetIsRunning true))

(fn InitAbility)

(fn CanStart
  (if (Variables|Default|GetIsRunning)
    (return false)
    (else
      (return true))))

(fn StopAbility
  (Variables|Default|SetIsRunning false))

(fn GetOwningComponent
  (bind _asbp_ability_component (Utilities|Casting|CastToBP_AbilityComponent (Utilities|GetOuterObject "BP_AbilityComponent")))
  (Utilities|IsValid _asbp_ability_component
    (:Is%20Valid
      (return _asbp_ability_component))
    (:Is%20Not%20Valid
      (Development|PrintString "Cast failed")
      (return 0))))