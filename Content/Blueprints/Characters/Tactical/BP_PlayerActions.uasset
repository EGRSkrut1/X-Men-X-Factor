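; Player action component for the tactical grid that tracks which tile the cursor is over and highlights it.
; On BeginPlay it finds the Bp_Grid actor in the level and stores a reference.
; UpdateTileUnderCursor asks the grid for the tile under the cursor and, when it changes, moves a tile state from the previous hovered tile to the new one.
; The Tick event is disabled, and nothing in this file calls the update.
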(event EventBeginPlay
  (bind _returnvalue (Actor|GetActorOfClass "/Game/Blueprints/Grid/Bp_Grid.Bp_Grid_C"))
  (Variables|Default|SetGrid _returnvalue))

(event EventTick
  (params (DeltaSeconds :type Float%20%28single-precision%29)))

(fn ConstructionScript)

(fn UpdateTileUnderCursor
  (bind _grid (Variables|Default|GetGrid))
  (bind _index (Default|GetTileIndexUnderCursor _grid))
  (if (!= _index (Variables|Default|GetHoveredTile))
    (Default|RemoveTileState (Variables|Default|GetGrid) (Variables|Default|GetHoveredTile) "NewEnumerator1")
    (bind _output_get (Variables|Default|SetHoveredTile _index))
    (Default|SetTileState _grid "NewEnumerator1" _output_get)))