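; Player controller for tactical mode that selects units and issues move orders with the mouse.
; Left click traces under the cursor, stores a hit BP_BaseUnit as the selection and notifies of the change, otherwise clears it.
; A hit unit gets ShowSelect, then Deselect right after the notification.
; Right click sends a selected BP_BaseTactical to the traced location via MoveToLocation and MoveToNextPoint, with debug prints throughout.
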(event Input|MouseEvents|LeftMouseButton
  (params (Key :type Key%20Structure :default "None"))
  ;[0.15 0.15 0.15 0.5] Choice unit
  (:Pressed
    (bind _asbp_base_unit (Utilities|Casting|CastToBP_BaseUnit (.HitActor (Collision|BreakHitResult (.HitResult (Game|Player|GetHitResultUnderCursorbyChannel (Game|GetPlayerController 0) "TraceTypeQuery1" true)))))
      (:then
        (bind _output_get (Variables|Default|SetCurrentSelectedUnit _asbp_base_unit))
        (Default|ShowSelect _output_get)
        (Default|CallOnSelectedUnitChanged)
        (Default|Deselect _output_get))
      (:CastFailed
        (Default|CallOnSelectedUnitChanged)
        (Variables|Default|SetCurrentSelectedUnit 0)))))

(event Input|MouseEvents|RightMouseButton
  (params (Key :type Key%20Structure :default "None"))
  (bind _returnvalue (Game|GetPlayerController 0))
  (bind _currentselectedunit (Variables|Default|GetCurrentSelectedUnit))
  (bind _hitresult (Game|Player|GetHitResultUnderCursorbyChannel _returnvalue "TraceTypeQuery3" true))
  (bind _location (Collision|BreakHitResult _hitresult))
  ;[0.15 0.15 0.15 0.5] Comment
  (:Pressed
    (Development|PrintString (Utilities|String|Append "Clcik right" " Location = " (Utilities|String|ToString(Vector) _location) " Cast = " (Utilities|GetDisplayName (stale _asbp_base_tactical))))
    (if (Utilities|IsValid _currentselectedunit)
      (bind _asbp_base_tactical (Utilities|Casting|CastToBP_BaseTactical _currentselectedunit))
      (Development|PrintString "move to location")
      (Default|MovetoLocation _asbp_base_tactical _location)
      (Development|PrintString "move to next point")
      (Default|MovetoNextPoint _asbp_base_tactical)
      (else
        (Development|PrintString "can't move")))))

(fn ConstructionScript)