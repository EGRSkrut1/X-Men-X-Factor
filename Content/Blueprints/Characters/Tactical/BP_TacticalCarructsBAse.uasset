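; Base Blueprint for tactical characters that can spend action points to use an ability.
; On BeginPlay it constructs an ability object and adds it to the ability list on XAbilityComponent.
; Pressing the AbilityPressE input clears targeting and, if any action points remain, starts the first ability and deducts two points.
; The check only requires points above zero, so the total can go negative.
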(event EventBeginPlay
  (bind _returnvalue (Game|ConstructObjectfromClass 0))
  (Utilities|Array|Add (Variables|Default|GetAbilities (Variables|Default|GetXAbilityComponent)) _returnvalue))

(event Input|ActionEvents|InputActionAbilityPressE
  (params (Key :type Key%20Structure))
  (:Pressed
    (Variables|Default|SetIsTargeting false)
    (if (> (Variables|Default|GetActionPoints) 0)
      (CallFunction|StartAbility (Utilities|Array|Get(acopy) (Variables|Default|GetAbilities (Variables|Default|GetXAbilityComponent))))
      (Variables|Default|SetActionPoints (- (Variables|Default|GetActionPoints) 2)))))

(fn ConstructionScript)