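; A grid action Blueprint for tactical mode that highlights the valid neighbours of a chosen tile.
; ExecuteAction clears one tile state across the grid, asks the grid's pathfinding for valid neighbours of the index, optionally including diagonals, and applies that state to each.
; When destroyed, it runs the action with an out-of-range index, which serves to clear the highlight.
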(event EventBeginPlay
  (|CallParentFunction) ; This node is disabled and will not be called.\nDrag off pins to build functionality.
)

(event Collision|EventActorBeginOverlap
  (params (OtherActor :type Actor%20Object%20Reference))
  (|CallParentFunction OtherActor) ; This node is disabled and will not be called.\nDrag off pins to build functionality.
)

(event EventTick
  (params (DeltaSeconds :type Float%20%28single-precision%29))
  (|CallParentFunction DeltaSeconds) ; This node is disabled and will not be called.\nDrag off pins to build functionality.
)

(event EventDestroyed
  (CallFunction|ExecuteAction (Utilities|Struct|MakeIntPoint -999 -999)))

(fn ConstructionScript
  (|CallParentFunction))

(fn ExecuteAction
  (params (Index :type Int%20Point%20Structure))
  (Default|ClearStatefromTiles (Variables|/Game/Blueprints/TacticalMode/BP_PlayerGridActions.BP_PlayerGridActions_C|GetGrid (Variables|Default|GetPlayerGridActions)) "NewEnumerator5")
  (bind _neighbours (Default|GetValidNeighbours (Variables|/Game/Blueprints/TacticalMode/Bp_Grid.BP_Grid_C|GetGridPathfinding (Variables|/Game/Blueprints/TacticalMode/BP_PlayerGridActions.BP_PlayerGridActions_C|GetGrid (Variables|Default|GetPlayerGridActions))) Index (Variables|Default|GetIncludeDiagonals)))
  (for _array_element _neighbours
    (Default|SetTileState (Variables|/Game/Blueprints/TacticalMode/BP_PlayerGridActions.BP_PlayerGridActions_C|GetGrid (Variables|Default|GetPlayerGridActions)) "NewEnumerator5" _array_element)))