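; Tactical-mode combat system that spawns units and tracks their placement on the grid.
; BeginPlay spawns Cyclop, Emma Frost and a melee enemy on hard-coded tiles through AddUnitOnTile, which registers each unit and passes it the Grid.
; SetUnitIndexOnGrid syncs tile occupancy with unit index and teleports the unit above its tile, or far away if none exists.
; RemoveUnitFromGrid unregisters the unit, moves it to a sentinel index and destroys it.
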(event EventBeginPlay
  (Utilities|FlowControl|Sequence
    (:then_0
      (bind _returnvalue (Game|SpawnActorfromClass "/Game/Blueprints/Characters/Tactical/Units/BP_UnitCyclop.BP_UnitCyclop_C" (Math|Transform|MakeTransform "0, 0, 0" "0, 0, 0" "1.000000,1.000000,1.000000") "AlwaysSpawn" "MultiplyWithRoot" 0 "NewEnumerator1" 0))
      (CallFunction|AddUnitonTile _returnvalue (Utilities|Struct|MakeIntPoint 14 39)))
    (:then_1
      (bind _returnvalue_2 (Game|SpawnActorfromClass "/Game/Blueprints/Characters/Tactical/Units/BP_UnitEmmaFrost.BP_UnitEmmaFrost_C" (Math|Transform|MakeTransform "0, 0, 0" "0, 0, 0" "1.000000,1.000000,1.000000") "AlwaysSpawn" "MultiplyWithRoot" 0 "NewEnumerator2" 0))
      (CallFunction|AddUnitonTile _returnvalue_2 (Utilities|Struct|MakeIntPoint 18 25)))
    (:then_2
      (bind _returnvalue_3 (Game|SpawnActorfromClass "/Game/Blueprints/Characters/Tactical/Enemy/BP_EnemyMelee.BP_EnemyMelee_C" (Math|Transform|MakeTransform "0, 0, 0" "0, 0, 0" "1.000000,1.000000,1.000000") "AlwaysSpawn" "MultiplyWithRoot" 0 "NewEnumerator0" 0))
      (CallFunction|AddUnitonTile _returnvalue_3 (Utilities|Struct|MakeIntPoint 7 22)))))

(fn ConstructionScript)

(fn AddUnitonTile
  (params (Unit :type BP%20Base%20Tactical%20Object%20Reference) (Index :type Int%20Point%20Structure))
  (Utilities|Array|Add (Variables|Default|GetUnitsOnGrid) Unit)
  (CallFunction|SetUnitIndexonGrid Unit Index)
  (Default|SetGrid Unit (Variables|Default|GetGrid)))

(fn SetUnitIndexonGrid
  (params (Unit :type BP%20Base%20Tactical%20Object%20Reference) (Index :type Int%20Point%20Structure))
  (Utilities|FlowControl|Sequence
    (:then_0
      (if (!= (Variables|/Game/Blueprints/Characters/Tactical/BP_BaseTactical.BP_BaseTactical_C|GetIndex Unit) Index)
        (Utilities|FlowControl|Sequence
          (:then_0
            (bind _output_get (LocalVariables|SetPreviousTile (.Value (Utilities|Map|Find (Variables|/Game/Blueprints/TacticalMode/Bp_Grid.BP_Grid_C|GetGridTiles (Variables|Default|GetGrid)) (Variables|/Game/Blueprints/Characters/Tactical/BP_BaseTactical.BP_BaseTactical_C|GetIndex Unit)))))
            (if (== (.UnitOnTile (Utilities|Struct|BreakS_TileData _output_get)) Unit)
              (bind _structout (Utilities|Struct|SetmembersinS_TileData (LocalVariables|GetPreviousTile)))
              (Utilities|Map|Add (Variables|/Game/Blueprints/TacticalMode/Bp_Grid.BP_Grid_C|GetGridTiles (Variables|Default|GetGrid)) (.Index (Utilities|Struct|BreakS_TileData _structout)) _structout)))
          (:then_1
            (Variables|/Game/Blueprints/Characters/Tactical/BP_BaseTactical.BP_BaseTactical_C|SetIndex Unit Index)
            (if (!= Index (Utilities|Struct|MakeIntPoint -999 -999))
              (bind _structout_2 (Utilities|Struct|SetmembersinS_TileData (.Value (Utilities|Map|Find (Variables|/Game/Blueprints/TacticalMode/Bp_Grid.BP_Grid_C|GetGridTiles (Variables|Default|GetGrid)) Index)) Unit))
              (Utilities|Map|Add (Variables|/Game/Blueprints/TacticalMode/Bp_Grid.BP_Grid_C|GetGridTiles (Variables|Default|GetGrid)) (.Index (Utilities|Struct|BreakS_TileData _structout_2)) _structout_2))))))
    (:then_1
      (Transformation|SetActorLocation Unit (Math|Vector|SelectVector (+ (.location (.Transform (Utilities|Struct|BreakS_TileData (.Value (Utilities|Map|Find (Variables|/Game/Blueprints/TacticalMode/Bp_Grid.BP_Grid_C|GetGridTiles (Variables|Default|GetGrid)) Index))))) "0.000000,0.000000,90.000000") "-999999.000000,-9999999.000000,-9999999.000000" (.ReturnValue (Utilities|Map|Find (Variables|/Game/Blueprints/TacticalMode/Bp_Grid.BP_Grid_C|GetGridTiles (Variables|Default|GetGrid)) Index))) false false))))

(fn RemoveUnitfromGrid
  (params (Unit :type BP%20Base%20Tactical%20Object%20Reference%20%28by%20ref%29))
  (Utilities|Array|RemoveItem (Variables|Default|GetUnitsOnGrid) Unit)
  (CallFunction|SetUnitIndexonGrid Unit (Utilities|Struct|MakeIntPoint -999 -999))
  (Actor|DestroyActor Unit))