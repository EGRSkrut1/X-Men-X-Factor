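; Tactical player controller that lets the player select units by clicking on them.
; On SelectAction press, it traces under the cursor on the Visibility channel and casts the hit actor to BP_BaseUnit.
; A hit unit becomes CurrentSelectedUnit and fires OnSelectedUnitChanged; any other result clears the selection without firing it.
; Debug prints report each click and its outcome.
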(event Input|ActionEvents|InputActionSelectAction
  (params (Key :type Key%20Structure :default "None"))
  (bind _returnvalue (Game|GetPlayerController 0))
  (bind _hitresult (Game|Player|GetHitResultUnderCursorbyChannel _returnvalue "TraceTypeQuery1" true))
  (bind _hitactor (Collision|BreakHitResult _hitresult))
  (:Pressed
    (Development|PrintString "Click")
    (bind _asbp_base_unit (Utilities|Casting|CastToBP_BaseUnit _hitactor)
      (:then
        (bind _output_get (Variables|Default|SetCurrentSelectedUnit _asbp_base_unit))
        (Default|CallOnSelectedUnitChanged)
        (Development|PrintString (Utilities|String|Append "Current selected unit = " (Utilities|GetDisplayName _output_get) " object = " (Utilities|GetDisplayName _hitactor))))
      (:CastFailed
        (Variables|Default|SetCurrentSelectedUnit 0)
        (Development|PrintString "cast failed")))))

(fn ConstructionScript)