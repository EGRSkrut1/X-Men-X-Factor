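; Grid generator actor that builds a field of static mesh tiles and highlights the one under the player's cursor.
; The construction script lays out tiles in nested X/Y loops with padding and a selectable Y offset; its component tag assignment is disconnected.
; Tick traces under the cursor, swapping the first "GridToMove"-tagged hit's material through a DoOnce, which restores and re-arms only upon hitting an untagged component.
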(event EventTick
  (params (DeltaSeconds :type Float%20%28single-precision%29))
  (bind _returnvalue (Game|GetPlayerController 0))
  (bind _hitresult (Game|Player|GetHitResultUnderCursorbyChannel _returnvalue "TraceTypeQuery1" true))
  (bind _hitcomponent (Collision|BreakHitResult _hitresult))
  (Utilities|IsValid _hitcomponent
    (:Is%20Valid
      (if (Components|ComponentHasTag _hitcomponent "GridToMove")
        (Utilities|FlowControl|DoOnce false :!label _label
          (:Completed
            (bind _output_get (Variables|Default|SetGridArray (Utilities|Array|MakeArray _hitcomponent)))
            (for _array_element _output_get
              (Rendering|Material|SetMaterial _array_element 0 "/Engine/MapTemplates/Materials/BasicAsset03.BasicAsset03"))))
        (else
          (for _array_element_2 (Variables|Default|GetGridArray)
            (Rendering|Material|SetMaterial _array_element_2 0 "/Engine/EditorLandscapeResources/AlphaBrushMaterial.AlphaBrushMaterial")
            (Utilities|Array|Clear (Variables|Default|GetGridArray))
            (goto _label Reset)))))))

(fn ConstructionScript
  (for _index (range 0 (Variables|Default|GetGridX))
    (for _index_2 (range 0 (Variables|Default|GetGridY))
      (bind _returnvalue (AddComponent|AddStaticMeshComponent false (Math|Transform|MakeTransform (Math|Vector|SelectVector (Math|Vector|MakeVector (* _index (Variables|Default|GetPaddingX)) (* _index_2 (Variables|Default|GetPaddingY)) 0.0) (Math|Vector|MakeVector (* _index (Variables|Default|GetPaddingX)) (+ (* _index_2 (Variables|Default|GetPaddingY)) (Variables|Default|GetOffset)) 0.0) false) "0, 0, 0" "1.000000,1.000000,1.000000"))))))