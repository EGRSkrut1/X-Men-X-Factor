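; BP_BaseEnemy is the base enemy for the tactical turn-based mode, with an HP widget and a placeholder turn.
; On BeginPlay it passes itself to its WBP_Enemy_HP widget as EnemyRef.
; TurnEnemy ignores its TargetActor and immediately calls FinishEnemyTurn, which checks the game mode's CurrentTurn, prints a message and switches to the player's turn.
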(event Custom|Event%20Turn%20Enemy
  (params (TargetActor :type Actor%20Object%20Reference))
  ;[0.15 0.15 0.15 0.5] Comment
  (CallFunction|FinishEnemyTurn))

(event EventBeginPlay
  (CallFunction|WidgetSpawn))

(fn ConstructionScript)

(fn WidgetSpawn
  ;[0.15 0.15 0.15 0.5] Widget
  (bind _aswbp_enemy_hp (Utilities|Casting|CastToWBP_Enemy_HP (UserInterface|GetUserWidgetObject (Variables|Default|GetHP_Widget))))
  (bind _asbp_base_enemy (Utilities|Casting|CastToBP_BaseEnemy self))
  (bind _output_get (Variables|/Game/UI/WBP_Enemy_HP.WBP_Enemy_HP_C|SetEnemy%20Ref _aswbp_enemy_hp _asbp_base_enemy))
  (return _output_get))

(fn FinishEnemyTurn
  ;[0.15 0.15 0.15 0.5] Comment
  (bind _asbp_game_mode_tactical (Utilities|Casting|CastToBP_GameMode_Tactical (Game|GetGameMode)))
  (if (Utilities|Enum|Equal(Enum) (Variables|/Game/Blueprints/TacticalMode/BP_GameMode_Tactical.BP_GameMode_Tactical_C|GetCurrentTurn _asbp_game_mode_tactical) "NewEnumerator1")
    (Development|PrintString "Finished the turn")
    (Default|SwitchtoPlayerTurn _asbp_game_mode_tactical)))