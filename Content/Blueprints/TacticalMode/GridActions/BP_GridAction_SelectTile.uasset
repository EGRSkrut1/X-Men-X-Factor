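; Tactical-mode grid action that toggles which tile is selected on the player's grid.
; ExecuteAction moves the selection tile state from PlayerGridActions.SelectedTile to the given index and stores that index.
; Passing the already selected tile clears its state and resets SelectedTile to the -999 sentinel index.
; When destroyed, the action executes with that sentinel index, removing any current selection.
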(event EventBeginPlay
  (|CallParentFunction) ; This node is disabled and will not be called.\nDrag off pins to build functionality.
)

(event Collision|EventActorBeginOverlap
  (params (OtherActor :type Actor%20Object%20Reference))
  (|CallParentFunction OtherActor) ; This node is disabled and will not be called.\nDrag off pins to build functionality.
)

(event EventTick
  (params (DeltaSeconds :type Float%20%28single-precision%29))
  (|CallParentFunction DeltaSeconds) ; This node is disabled and will not be called.\nDrag off pins to build functionality.
)

(event EventDestroyed
  (CallFunction|ExecuteAction (Utilities|Struct|MakeIntPoint -999 -999)))

(fn ConstructionScript
  (|CallParentFunction))

(fn ExecuteAction
  (params (Index :type Int%20Point%20Structure))
  (bind _playergridactions (Variables|Default|GetPlayerGridActions))
  (bind _playergridactions_2 (Variables|Default|GetPlayerGridActions))
  (bind _playergridactions_3 (Variables|Default|GetPlayerGridActions))
  (if (!= (Variables|/Game/Blueprints/TacticalMode/BP_PlayerGridActions.BP_PlayerGridActions_C|GetSelectedTile (Variables|Default|GetPlayerGridActions)) Index)
    (Default|RemoveTileState (Variables|/Game/Blueprints/TacticalMode/BP_PlayerGridActions.BP_PlayerGridActions_C|GetGrid _playergridactions) (Variables|/Game/Blueprints/TacticalMode/BP_PlayerGridActions.BP_PlayerGridActions_C|GetSelectedTile _playergridactions) "NewEnumerator2")
    (Variables|/Game/Blueprints/TacticalMode/BP_PlayerGridActions.BP_PlayerGridActions_C|SetSelectedTile (Variables|Default|GetPlayerGridActions) Index)
    (Default|SetTileState (Variables|/Game/Blueprints/TacticalMode/BP_PlayerGridActions.BP_PlayerGridActions_C|GetGrid _playergridactions_2) "NewEnumerator2" (Variables|/Game/Blueprints/TacticalMode/BP_PlayerGridActions.BP_PlayerGridActions_C|GetSelectedTile _playergridactions_2))
    (else
      (Default|RemoveTileState (Variables|/Game/Blueprints/TacticalMode/BP_PlayerGridActions.BP_PlayerGridActions_C|GetGrid _playergridactions_3) (Variables|/Game/Blueprints/TacticalMode/BP_PlayerGridActions.BP_PlayerGridActions_C|GetSelectedTile _playergridactions_3) "NewEnumerator2")
      (Variables|/Game/Blueprints/TacticalMode/BP_PlayerGridActions.BP_PlayerGridActions_C|SetSelectedTile (Variables|Default|GetPlayerGridActions) (Utilities|Struct|MakeIntPoint -999 -999)))))