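; Tactical-mode game mode that alternates turns between player units and enemies.
; Construction counts both sides, and finished-unit reports are compared against those totals to switch turns.
; Switching to the player turn resets the enemy count, restores player squad action points and calls OnTurnChanged.
; Switching to the enemy turn only sets the turn and fetches enemies; its stun check and OnTurnChanged call are disconnected.
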(fn ConstructionScript
  ;[0.15 0.15 0.15 0.5] Comment
  (CallFunction|UnitCounter)
  (CallFunction|EnemyCounter))

(fn PlayerUnitFinished
  (params (InSlotIndex :type Integer))
  (bind _finishedplayerslots (Variables|Default|GetFinishedPlayerSlots))
  (bind _totalplayerunits (Variables|Default|GetTotalPlayerUnits))
  (bind _returnvalue (Utilities|Array|Length _finishedplayerslots))
  ;[0.15 0.15 0.15 0.5] Comment
  (Development|PrintString (Utilities|String|Append "in slot index = " (Utilities|String|ToString(Integer) InSlotIndex)))
  (Utilities|Array|Add _finishedplayerslots InSlotIndex)
  (Development|PrintString (Utilities|String|Append "length" (Utilities|String|ToString(Integer) _returnvalue) "total player units" (Utilities|String|ToString(Integer) _totalplayerunits)))
  (if (== _returnvalue _totalplayerunits)
    (Development|PrintString "switch to enemy turn")
    (CallFunction|SwitchtoEnemyTurn)
    (Utilities|Array|Clear _finishedplayerslots)))

(fn EnemyUnitFinished
  ;[0.15 0.15 0.15 0.5] Comment
  (bind _result (Math|Integer|IncrementInt (Variables|Default|GetEnemyFinishedCount))
    (:%20%20
      (Variables|Default|SetEnemyFinishedCount _result)
      (if (>= (Variables|Default|GetEnemyFinishedCount) (Variables|Default|GetTotalEnemyUnits))
        (CallFunction|SwitchtoPlayerTurn)))))

(fn SwitchtoEnemyTurn
  (Variables|Default|SetCurrentTurn "NewEnumerator1")
  (bind _outactors (Actor|GetAllActorsOfClass "/Game/Blueprints/Characters/Tactical/Enemy/BP_BaseEnemy.BP_BaseEnemy_C")))

(fn SwitchtoPlayerTurn
  ;[0.15 0.15 0.15 0.5] Comment
  (Variables|Default|SetCurrentTurn "NewEnumerator0")
  (Variables|Default|SetEnemyFinishedCount 0)
  (CallFunction|RestorePlayerUnitsAP)
  (Default|CallOnTurnChanged)
  (bind _outactors (Actor|GetAllActorsOfClass "/Game/Blueprints/Characters/Tactical/Units/BP_BaseUnit.BP_BaseUnit_C"))
  (for _array_element _outactors
    ;[0.15 0.15 0.15 0.5] исправишь сам
    (if (Class|XAttributeComponent|IsinPlayerSquad (Actor|GetComponentbyClass _array_element "/Script/Xmen_Xfactor.XAttributeComponent"))
      _)))

(fn RestorePlayerUnitsAP
  (bind _outactors (Actor|GetAllActorsOfClass "/Script/Xmen_Xfactor.XTacticalCharacter"))
  (for _array_element _outactors
    ;[0.15 0.15 0.15 0.5] исправить на адекватное доставание аттрибут компонента
    (if (Class|XAttributeComponent|IsinPlayerSquad (Actor|GetComponentbyClass _array_element "/Script/Xmen_Xfactor.XAttributeComponent"))
      (Class|XAttributeComponent|ApplyActionPointsChange (Actor|GetComponentbyClass _array_element "/Script/Xmen_Xfactor.XAttributeComponent") (Variables|/Script/Xmen_Xfactor.XAttributeComponent|GetMaxActionPoints (Actor|GetComponentbyClass _array_element "/Script/Xmen_Xfactor.XAttributeComponent"))))))

(fn EnemyCounter
  ;[0.15 0.15 0.15 0.5] зачем это вообще надо? можно же просто брать размер массива O_о
  (bind _outactors (Actor|GetAllActorsOfClass "/Game/Blueprints/Characters/Tactical/Enemy/BP_BaseEnemy.BP_BaseEnemy_C"))
  (for _array_element _outactors
    (bind _result (Math|Integer|IncrementInt (LocalVariables|GetTemp%20Counter))
      (:%20%20
        (LocalVariables|SetTemp%20Counter _result))))
  (Variables|Default|SetTotalEnemyUnits (LocalVariables|GetTemp%20Counter)))

(fn UnitCounter
  ;[0.15 0.15 0.15 0.5] Comment
  (bind _outactors (Actor|GetAllActorsOfClass "/Game/Blueprints/Characters/Tactical/Units/BP_BaseUnit.BP_BaseUnit_C"))
  (for _array_element _outactors
    (bind _result (Math|Integer|IncrementInt (LocalVariables|GetTemp%20Counter))
      (:%20%20
        (LocalVariables|SetTemp%20Counter _result))))
  (Variables|Default|SetTotalPlayerUnits (LocalVariables|GetTemp%20Counter)))