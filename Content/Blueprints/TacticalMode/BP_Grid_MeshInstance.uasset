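; Tactical-mode grid visual actor that draws cells through one InstancedStaticMesh, with mesh, material, color and collision set on init.
; A parallel InstanceIndecies array maps cell indices to instances, so re-adding a cell replaces its instance.
; The first match among Normal, Hovered and IsNeighbour states sets RGB and a fill flag as custom data.
; The fill flag write omits the instance index, unlike the RGB writes.
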(event EventBeginPlay
  (Actor|Tick|SetActorTickEnabled false))

(fn ConstructionScript)

(fn AddInstance
  (params (Index :type Int%20Point%20Structure%20%28by%20ref%29) (InstanceTransform :type Transform%20%28by%20ref%29) (States :type Array%20of%20E_TileState%20Enums :default "NewEnumerator0"))
  (CallFunction|RemoveInstance Index)
  (Components|InstancedStaticMesh|AddInstance (Variables|Default|GetInstancedStaticMesh) InstanceTransform false)
  (bind _returnvalue (Utilities|Array|Add (Variables|Default|GetInstanceIndecies) Index))
  (LocalVariables|Seti _returnvalue)
  (bind (_color _isfilled) (CallFunction|GetColorfromStates States))
  (Components|InstancedStaticMesh|SetCustomDataValue (Variables|Default|GetInstancedStaticMesh) (LocalVariables|Geti) 0 (.R (Math|Color|BreakColor _color)) false)
  (Components|InstancedStaticMesh|SetCustomDataValue (Variables|Default|GetInstancedStaticMesh) (LocalVariables|Geti) 1 (.G (Math|Color|BreakColor _color)) false)
  (Components|InstancedStaticMesh|SetCustomDataValue (Variables|Default|GetInstancedStaticMesh) (LocalVariables|Geti) 2 (.B (Math|Color|BreakColor _color)) false)
  (Components|InstancedStaticMesh|SetCustomDataValue (Variables|Default|GetInstancedStaticMesh) 0 3 _isfilled false))

(fn RemoveInstance
  (params (Index :type Int%20Point%20Structure%20%28by%20ref%29))
  (bind _instanceindecies (Variables|Default|GetInstanceIndecies))
  (if (Utilities|Array|ContainsItem _instanceindecies Index)
    (Class|InstancedStaticMeshComponent|RemoveInstance (Variables|Default|GetInstancedStaticMesh) (Utilities|Array|FindItem _instanceindecies Index))
    (Utilities|Array|RemoveItem (Variables|Default|GetInstanceIndecies) Index)))

(fn ClearInstances
  (Components|InstancedStaticMesh|ClearInstances (Variables|Default|GetInstancedStaticMesh))
  (Utilities|Array|Clear (Variables|Default|GetInstanceIndecies)))

(fn InitGridMeshInstance
  (params (NewMesh :type Static%20Mesh%20Object%20Reference) (Material :type Material%20Interface%20Object%20Reference) (InLinearColor :type Linear%20Color%20Structure) (NewType :type ECollisionEnabled%20Enum :default "NoCollision"))
  (bind _instancedstaticmesh (Variables|Default|GetInstancedStaticMesh))
  (Components|StaticMesh|SetStaticMesh _instancedstaticmesh NewMesh)
  (Rendering|Material|SetMaterial _instancedstaticmesh 0 Material)
  (Rendering|Material|SetVectorParameterValueonMaterials (Variables|Default|GetInstancedStaticMesh) "Color" (Math|Conversions|ToVector(LinearColor) InLinearColor))
  (Collision|SetCollisionEnabled (Variables|Default|GetInstancedStaticMesh) NewType))

(fn GetColorfromStates
  (params (States :type Array%20of%20E_TileState%20Enums :default "NewEnumerator0"))
  (if (Utilities|Array|IsEmpty States)
    (return "" 0.0)
    (else
      (for _array_element (Utilities|Array|MakeArray "NewEnumerator0" "NewEnumerator1" "NewEnumerator5")
        (if (Utilities|Array|ContainsItem States _array_element)
          (return (Utilities|Select :Index _array_element :NewEnumerator0 "" :NewEnumerator1 "(R=1.000000,G=0.948275,B=0.302083,A=1.000000)" :NewEnumerator2 "(R=1.000000,G=0.184035,B=0.000000,A=1.000000)" :NewEnumerator3 "" :NewEnumerator4 "" :NewEnumerator5 "(R=1.000000,G=0.063984,B=0.749451,A=1.000000)") 1.0)))
      (return "" 0.0))))