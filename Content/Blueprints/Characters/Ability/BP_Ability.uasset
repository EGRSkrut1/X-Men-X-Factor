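; BP_Ability is a base ability object that tracks whether it is running.
; StartAbility and StopAbility set and clear IsRunning, CanStart allows a start only while it is not running, and InitAbility is an empty hook.
; GetOwningComponent finds the owning BP_AbilityComponent through the object's outer, printing an error if the cast result is invalid.
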(fn StartAbility
  (Variables|Default|SetIsRunning true))

(fn InitAbility)

(fn CanStart
  (if (Variables|Default|GetIsRunning)
    (return false)
    (else
      (return true))))

(fn StopAbility
  (Variables|Default|SetIsRunning false))

(fn GetOwningComponent
  (bind _asbp_ability_component (Utilities|Casting|CastToBP_AbilityComponent (Utilities|GetOuterObject "/Game/Blueprints/Characters/Ability/BP_AbilityComponent.BP_AbilityComponent")))
  (Utilities|IsValid _asbp_ability_component
    (:Is%20Valid
      (return _asbp_ability_component))
    (:Is%20Not%20Valid
      (Development|PrintString 0 "Cast failed")
      (return 0))))