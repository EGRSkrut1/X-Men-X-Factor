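; Grid action for tactical mode that spawns a unit and places it on a grid tile.
; ExecuteAction checks the index against the PlayerGridActions grid, then spawns a BP_BaseUnit with the action's UnitType using AlwaysSpawn collision handling.
; The new unit is handed to the CombatSystem's AddUnitOnTile to register it on that tile.
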(event EventBeginPlay
  (|CallParentFunction) ; This node is disabled and will not be called.\nDrag off pins to build functionality.
)

(event Collision|EventActorBeginOverlap
  (params (OtherActor :type Actor%20Object%20Reference))
  (|CallParentFunction OtherActor) ; This node is disabled and will not be called.\nDrag off pins to build functionality.
)

(event EventTick
  (params (DeltaSeconds :type Float%20%28single-precision%29))
  (|CallParentFunction DeltaSeconds) ; This node is disabled and will not be called.\nDrag off pins to build functionality.
)

(fn ConstructionScript
  (|CallParentFunction))

(fn ExecuteAction
  (params (Index :type Int%20Point%20Structure))
  (if (Default|IsValidGridIndex (Variables|/Game/Blueprints/TacticalMode/BP_PlayerGridActions.BP_PlayerGridActions_C|GetGrid (Variables|Default|GetPlayerGridActions)) Index)
    (bind _returnvalue (Game|SpawnActorfromClass "/Game/Blueprints/Characters/Tactical/Units/BP_BaseUnit.BP_BaseUnit_C" (Math|Transform|MakeTransform "0, 0, 0" "0, 0, 0" "1.000000,1.000000,1.000000") "AlwaysSpawn" "MultiplyWithRoot" 0 (Variables|Default|GetUnitType) 0))
    (Default|AddUnitonTile (Variables|/Game/Blueprints/TacticalMode/BP_PlayerGridActions.BP_PlayerGridActions_C|GetCombatSystem (Variables|Default|GetPlayerGridActions)) _returnvalue Index)))