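; Grid pathfinder for tactical mode that runs A* between two tiles and returns the route, excluding the start.
; Neighbours come from hexagon offsets (the only shape handled) and are filtered by height difference, with walkability checked only for start and target.
; Discovered tiles stay in parallel arrays sorted by cost plus a Manhattan or diagonal estimate.
; The search stops when the target is discovered, then traces previous indexes back.
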(fn ConstructionScript)

(fn GetNeighboursIndexes
  (params (Index :type Int%20Point%20Structure) (IncludeDiagonals :type Boolean))
  (switch Utilities|FlowControl|Switch|SwitchonE_GridShape (Variables|/Game/Blueprints/TacticalMode/Bp_Grid.BP_Grid_C|GetGrid%20Shape (Variables|Default|GetGrid))
    (:NewEnumerator0
      (return (CallFunction|GetNeighbourIndexesforHexagon Index)))))

(fn GetNeighbourIndexesforHexagon
  (params (Index :type Int%20Point%20Structure))
  (return (Utilities|Array|MakeArray (+ Index (Utilities|Struct|MakeIntPoint 1 1)) (+ Index (Utilities|Struct|MakeIntPoint 0 2)) (+ Index (Utilities|Struct|MakeIntPoint -1 1)) (+ Index (Utilities|Struct|MakeIntPoint -1 -1)) (+ Index (Utilities|Struct|MakeIntPoint 0 -2)) (+ Index (Utilities|Struct|MakeIntPoint 1 -1)))))

(fn GetValidNeighboursIndexes
  (params (Index :type Int%20Point%20Structure) (IncludeDiagonals :type Boolean))
  (LocalVariables|SetInputData (.Value (Utilities|Map|Find (Variables|/Game/Blueprints/TacticalMode/Bp_Grid.BP_Grid_C|GetGridTiles (Variables|Default|GetGrid)) Index)))
  (bind _neighbours (CallFunction|GetNeighboursIndexes Index IncludeDiagonals))
  (for _array_element _neighbours
    (LocalVariables|SetData (.Value (Utilities|Map|Find (Variables|/Game/Blueprints/TacticalMode/Bp_Grid.BP_Grid_C|GetGridTiles (Variables|Default|GetGrid)) _array_element)))
    (if (<= (Math|Float|Absolute(Float) (- (.z (.location (.transform (LocalVariables|GetData)))) (.z (.location (.transform (LocalVariables|GetInputData)))))) (.z (Variables|/Game/Blueprints/TacticalMode/Bp_Grid.BP_Grid_C|GetGrid%20Tile%20Size (Variables|Default|GetGrid))))
      ;[0.15 0.15 0.15 0.5] Neighbour
      (Utilities|Array|Add (LocalVariables|GetReturnArray) (Utilities|Struct|MakeS_PathfindingData (.index (LocalVariables|GetData)) 1 99999 99999 Index))))
  (return (LocalVariables|GetReturnArray)))

(fn FindPath
  (params (Start :type Int%20Point%20Structure) (TargetDestination :type Int%20Point%20Structure) (Diagonals :type Boolean))
  (Variables|Default|SetStartIndex Start)
  (Variables|Default|SetTargetIndex TargetDestination)
  (Variables|Default|SetIncludeDiagonals Diagonals)
  (CallFunction|ClearGeneratedData)
  (bind _isvalid (CallFunction|IsInputDataValid))
  (if _isvalid
    (CallFunction|DiscoverTile (Utilities|Struct|MakeS_PathfindingData (Variables|Default|GetStartIndex) 1 0 (CallFunction|GetMinimunCostBetweenTwoTiles (Variables|Default|GetStartIndex) (Variables|Default|GetTargetIndex) (Variables|Default|GetIncludeDiagonals)) "(X=-999,Y=-999)"))
    (while (> (Utilities|Array|Length (Variables|Default|GetDiscoveredTilesIndexes)) 0)
      (bind _foundtargettile (CallFunction|AnalyseNextDiscoveredTile))
      (if _foundtargettile
        (bind _path (CallFunction|GeneratePath))
        (return _path)))
    ;[0.15 0.15 0.15 0.5] no path found
    (return (Utilities|Array|MakeArray ""))
    (else
      (return (Utilities|Array|MakeArray "")))))

(fn IsInputDataValid
  (if (!= (Variables|Default|GetStartIndex) (Variables|Default|GetTargetIndex))
    (if (and (Default|IsTileWalkable (Variables|Default|GetGrid) (Variables|Default|GetStartIndex)) (Default|IsTileWalkable (Variables|Default|GetGrid) (Variables|Default|GetTargetIndex)))
      (return true)
      (else
        (return false)))
    (else
      ;[0.15 0.15 0.15 0.5] we dont have to do any pathfinding because were already in target
      (return false))))

(fn DiscoverTile
  (params (TilePathData :type S%20Pathfinding%20Data%20Structure))
  (Utilities|Map|Add (Variables|Default|GetPathfindingData) (.Index (Utilities|Struct|BreakS_PathfindingData TilePathData)) TilePathData)
  (CallFunction|InserTileinDiscoveredArray TilePathData))

(fn GetMinimunCostBetweenTwoTiles
  (params (Index1 :type Int%20Point%20Structure) (Index2 :type Int%20Point%20Structure) (Diagonals :type Boolean))
  (bind _returnvalue (- Index1 Index2))
  (bind _returnvalue_2 (- Index1 Index2))
  ;[0.15 0.15 0.15 0.5] works worse for hexagon. better works with square
  ;;[0.15 0.15 0.15 0.5] AKA manhattan distance
  (if Diagonals
    (return (Math|Integer|Max(Integer) (Math|Integer|Absolute(Integer) (.x _returnvalue_2)) (Math|Integer|Absolute(Integer) (.y _returnvalue_2))))
    (else
      (return (+ (Math|Integer|Absolute(Integer) (.x _returnvalue)) (Math|Integer|Absolute(Integer) (.y _returnvalue)))))))

(fn AnalyseNextDiscoveredTile
  (bind _tilepathdata (CallFunction|PullCheapestTileOutOfDescoveredList))
  (bind _output_get (Variables|Default|SetCurrentDiscoveredTile _tilepathdata))
  (bind _neighbours (CallFunction|GetValidNeighboursIndexes (.Index (Utilities|Struct|BreakS_PathfindingData _output_get)) (Variables|Default|GetIncludeDiagonals)))
  (bind _output_get_2 (Variables|Default|SetCurrentNeighbours _neighbours))
  (while (> (Utilities|Array|Length _output_get_2) 0)
    (bind _istargettile (CallFunction|DiscoverNextNeighbour))
    (if _istargettile
      (return true)))
  ;[0.15 0.15 0.15 0.5] none of the neighbours were the target
  (return false))

(fn GeneratePath
  (LocalVariables|SetCurrentIndex (Variables|Default|GetTargetIndex))
  (while (!= (LocalVariables|GetCurrentIndex) (Variables|Default|GetStartIndex))
    (Utilities|Array|Add (LocalVariables|GetInvertedPath) (LocalVariables|GetCurrentIndex))
    (LocalVariables|SetCurrentIndex (.PreviousIndex (Utilities|Struct|BreakS_PathfindingData (.Value (Utilities|Map|Find (Variables|Default|GetPathfindingData) (LocalVariables|GetCurrentIndex)))))))
  (bind _arrayelement (Utilities|Array|ReverseforEachLoop (LocalVariables|GetInvertedPath))
    (:LoopBody
      (Utilities|Array|Add (LocalVariables|GetReturnArray) _arrayelement))
    (:Completed
      (return (LocalVariables|GetReturnArray)))))

(fn PullCheapestTileOutOfDescoveredList
  (LocalVariables|SetTileIndex (Utilities|Array|Get(acopy) (Variables|Default|GetDiscoveredTilesIndexes)))
  (Utilities|Array|RemoveIndex (Variables|Default|GetDiscoveredTileSortingCosts))
  (Utilities|Array|RemoveIndex (Variables|Default|GetDiscoveredTilesIndexes))
  (Utilities|Array|Add (Variables|Default|GetAnalysedTilesIndexes) (LocalVariables|GetTileIndex))
  (return (.Value (Utilities|Map|Find (Variables|Default|GetPathfindingData) (LocalVariables|GetTileIndex)))))

(fn DiscoverNextNeighbour
  (bind _targetindex (Variables|Default|GetTargetIndex))
  (Variables|Default|SetCurrentNeighbour (Utilities|Array|Get(acopy) (Variables|Default|GetCurrentNeighbours)))
  ;[0.15 0.15 0.15 0.5] delete first neighbour from neighbours array because we dont need it anymore. were gonna analyse it tho
  (Utilities|Array|RemoveIndex (Variables|Default|GetCurrentNeighbours))
  (if (not (Utilities|Array|ContainsItem (Variables|Default|GetAnalysedTilesIndexes) (.Index (Utilities|Struct|BreakS_PathfindingData (Variables|Default|GetCurrentNeighbour)))))
    ;[0.15 0.15 0.15 0.5] if player walked 10 units and current neighbour cost is 2 => Cost from Start = 12
    (LocalVariables|SetCostFromStart (+ (.CostFromStart (Utilities|Struct|BreakS_PathfindingData (Variables|Default|GetCurrentDiscoveredTile))) (.ColorToEnterTile (Utilities|Struct|BreakS_PathfindingData (Variables|Default|GetCurrentNeighbour)))))
    ;[0.15 0.15 0.15 0.5] in case neighbour is already in list
    (bind _output_get (LocalVariables|SetIndexInDiscovered (Utilities|Array|FindItem (Variables|Default|GetDiscoveredTilesIndexes) (.Index (Utilities|Struct|BreakS_PathfindingData (Variables|Default|GetCurrentNeighbour))))))
    ;[0.15 0.15 0.15 0.5] is neighbour new?
    (if (== _output_get -1)
      _
      (else
        (bind _output_get_2 (Variables|Default|SetCurrentNeighbour (.Value (Utilities|Map|Find (Variables|Default|GetPathfindingData) (.Index (Utilities|Struct|BreakS_PathfindingData (Variables|Default|GetCurrentNeighbour)))))))
        ;[0.15 0.15 0.15 0.5] have we found faster route to neighbour?
        (if (< (LocalVariables|GetCostFromStart) (.CostFromStart (Utilities|Struct|BreakS_PathfindingData _output_get_2)))
          (Utilities|Array|RemoveIndex (Variables|Default|GetDiscoveredTilesIndexes) (LocalVariables|GetIndexInDiscovered))
          (Utilities|Array|RemoveIndex (Variables|Default|GetDiscoveredTileSortingCosts) (LocalVariables|GetIndexInDiscovered))
          (else
            (return false)))))
    (CallFunction|DiscoverTile (Utilities|Struct|MakeS_PathfindingData (.Index (Utilities|Struct|BreakS_PathfindingData (Variables|Default|GetCurrentNeighbour))) (.ColorToEnterTile (Utilities|Struct|BreakS_PathfindingData (Variables|Default|GetCurrentNeighbour))) (LocalVariables|GetCostFromStart) (CallFunction|GetMinimunCostBetweenTwoTiles (.Index (Utilities|Struct|BreakS_PathfindingData (Variables|Default|GetCurrentNeighbour))) (Variables|Default|GetTargetIndex) (Variables|Default|GetIncludeDiagonals)) (.Index (Utilities|Struct|BreakS_PathfindingData (Variables|Default|GetCurrentDiscoveredTile)))))
    (if (and (== (.x (.Index (Utilities|Struct|BreakS_PathfindingData (Variables|Default|GetCurrentNeighbour)))) (.x _targetindex)) (== (.y (.Index (Utilities|Struct|BreakS_PathfindingData (Variables|Default|GetCurrentNeighbour)))) (.y _targetindex)))
      (return true)
      (else
        (return false)))
    (else
      (return false))))

(fn InserTileinDiscoveredArray
  (params (TileData :type S%20Pathfinding%20Data%20Structure))
  (bind (_index _colortoentertile _costfromstart _minimumcosttotarget) (Utilities|Struct|BreakS_PathfindingData TileData))
  (bind _discoveredtilesortingcosts (Variables|Default|GetDiscoveredTileSortingCosts))
  (bind _discoveredtilesortingcosts_2 (Variables|Default|GetDiscoveredTileSortingCosts))
  (LocalVariables|SetSortingCost (+ _costfromstart _minimumcosttotarget))
  ;[0.15 0.15 0.15 0.5] if array is empty
  (if (== (Utilities|Array|Length _discoveredtilesortingcosts) 0)
    ;[0.15 0.15 0.15 0.5] we adding adding it to DiscoveredTilesIndexes without checking for cost
    (Utilities|Array|Add _discoveredtilesortingcosts (LocalVariables|GetSortingCost) :!label _label)
    (Utilities|Array|Add (Variables|Default|GetDiscoveredTilesIndexes) (.Index (Utilities|Struct|BreakS_PathfindingData TileData)))
    (else
      ;[0.15 0.15 0.15 0.5] we have to make sure that were inserting the cheaper than the previous one
      (if (>= (LocalVariables|GetSortingCost) (Utilities|Array|Get(acopy) _discoveredtilesortingcosts_2 (Utilities|Array|LastIndex _discoveredtilesortingcosts_2)))
        (goto _label)
        (else
          ;[0.15 0.15 0.15 0.5] VERY EXPENSIVE
          (bind (_array_element _array_index) (Utilities|Array|ForEachLoopwithBreak (Variables|Default|GetDiscoveredTileSortingCosts) :!label _label_2)
            (:LoopBody
              ;[0.15 0.15 0.15 0.5] true means the cost of element is HIGHER than the cost of current tile
              (if (>= _array_element (LocalVariables|GetSortingCost))
                (Utilities|Array|Insert (Variables|Default|GetDiscoveredTileSortingCosts) (LocalVariables|GetSortingCost) _array_index)
                (Utilities|Array|Insert (Variables|Default|GetDiscoveredTilesIndexes) (.Index (Utilities|Struct|BreakS_PathfindingData TileData)) _array_index)
                (goto _label_2 Break)))))))))

(fn ClearGeneratedData
  (Utilities|Map|Clear (Variables|Default|GetPathfindingData))
  (Utilities|Array|Clear (Variables|Default|GetDiscoveredTileSortingCosts))
  (Utilities|Array|Clear (Variables|Default|GetDiscoveredTilesIndexes))
  (Utilities|Array|Clear (Variables|Default|GetAnalysedTilesIndexes)))