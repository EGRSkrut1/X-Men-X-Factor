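; Cyclops laser ability that damages enemies lying along a direction on the tile grid.
; StartAbility derives a normalized direction from the owner's tile and the stored TargetTile, then updates TargetTile from the cursor.
; Over LaserLength iterations, it compares every BP_BaseEnemy's tile with the start offset by direction times that enemy's array index, not the laser step.
; Matches take damage through their AttributeComponent and call StopAbility.
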(event EventBeginPlay
  (|CallParentFunction) ; This node is disabled and will not be called.\nDrag off pins to build functionality.
)

(event EventTick
  (params (DeltaSeconds :type Float%20%28single-precision%29))
  (|CallParentFunction DeltaSeconds) ; This node is disabled and will not be called.\nDrag off pins to build functionality.
)

(fn StartAbility
  (bind _grid (Variables|Default|GetGrid))
  (|CallParentFunction)
  (bind _abilitycomponent (CallFunction|GetOwningComponent))
  (bind _index (Default|GetTileIndexfromWorldLocation (Variables|Default|GetGrid) (Transformation|GetActorLocation (Variables|/Game/Blueprints/Characters/Ability/BP_AbilityComponent.BP_AbilityComponent_C|GetOwnerActor _abilitycomponent))))
  (bind _output_get (Variables|Default|SetStartTile _index))
  (Variables|Default|SetDirection (Class|KismetMathLibrary|VectorNormal2D (Math|Vector|MakeVector (Math|Conversions|ToFloat(Integer) (.X (Utilities|Struct|BreakIntPoint (- _output_get (Variables|Default|GetTargetTile))))) (Math|Conversions|ToFloat(Integer) (.Y (Utilities|Struct|BreakIntPoint (- _output_get (Variables|Default|GetTargetTile))))) 0.0) 0.0001))
  (bind _location (Default|GetCursorLocationonGrid _grid))
  (bind _index_2 (Default|GetTileIndexfromWorldLocation _grid _location))
  (Variables|Default|SetTargetTile _index_2)
  (for _index_3 (range 0 (Variables|Default|GetLaserLength))
    (bind _outactors (Actor|GetAllActorsOfClass "/Game/Blueprints/Characters/Tactical/Enemy/BP_BaseEnemy.BP_BaseEnemy_C"))
    (for (_array_element _array_index) _outactors
      (bind _index_4 (Default|GetTileIndexfromWorldLocation (Variables|Default|GetGrid) (Transformation|GetActorLocation _array_element)))
      (if (and (== (+ (* (.X (Math|Vector|BreakVector (Variables|Default|GetDirection))) _array_index) (.X (Utilities|Struct|BreakIntPoint (Variables|Default|GetStartTile)))) (.X (Utilities|Struct|BreakIntPoint _index_4))) (== (+ (* (.Y (Math|Vector|BreakVector (Variables|Default|GetDirection))) _array_index) (.Y (Utilities|Struct|BreakIntPoint (Variables|Default|GetStartTile)))) (.Y (Utilities|Struct|BreakIntPoint _index_4))))
        (bind _asbp_base_enemy (Utilities|Casting|CastToBP_BaseEnemy _array_element))
        (Class|XAttributeComponent|ApplyDamage (Variables|/Script/Xmen_Xfactor.XTacticalCharacter|GetAttributeComponent _asbp_base_enemy) (Variables|Default|GetDamage))
        (CallFunction|StopAbility)))))