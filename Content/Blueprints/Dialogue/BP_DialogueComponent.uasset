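; Dialogue component that runs data-table-driven conversations through a WBP_Dialogue widget.
; Interact creates the widget and shows the cursor, advances the text on later calls, and closes it once the end flag is set.
; Each row names the next row and table, chaining the conversation.
; Open-ended choices, built only when the widget is created, become WBP_Option children that receive the component; OptionSelected clears them and jumps to the given row.
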(event Custom|Option%20Selected
  (params (DataTable :type Data%20Table%20Object%20Reference) (RowName :type Name))
  ;[0.15 0.15 0.15 0.5] Comment
  (bind _returnvalue (Utilities|GetDataTableRow DataTable RowName)
    (:then
      (Widget|Panel|ClearChildren (Variables|/Game/UI/Widgets/WBP_Dialogue.WBP_Dialogue_C|GetScrollBox_1 (Variables|Default|GetDialogueWidget)))
      (Default|UpdateDialogue (Variables|Default|GetDialogueWidget) (.Dialogue (Utilities|Struct|BreakS_Dialogue _returnvalue)))
      (Variables|Default|SetRow%20Name (.Row (Utilities|Struct|BreakS_Dialogue _returnvalue)))
      (Variables|Default|SetData%20Table (.DataTable (Utilities|Struct|BreakS_Dialogue _returnvalue)))
      (Variables|Default|SetEndDialogue (.EndDialogue (Utilities|Struct|BreakS_Dialogue _returnvalue))))))

(event EventInteract
  (params (playerref :type BP%20Cyclop%20Object%20Reference))
  (bind _returnvalue (Game|GetPlayerController 0))
  (bind _returnvalue_2 (Game|GetPlayerController 0))
  ;[0.15 0.15 0.15 0.5] Comment
  (if (Variables|Default|GetEndDialogue)
    ;;[0.15 0.15 0.15 0.5] Comment
    (Widget|RemovefromParent (Variables|Default|GetDialogueWidget))
    (Variables|Default|SetDialogueWidget 0)
    ;;[0.15 0.15 0.15 0.5] Comment
    (Input|SetInputModeGameOnly _returnvalue_2 false)
    (Variables|/Script/Engine.PlayerController|SetbShowMouseCursor _returnvalue_2 false)
    (else
      (Utilities|IsValid (Variables|Default|GetDialogueWidget)
        (:Is%20Valid
          ;;[0.15 0.15 0.15 0.5] Comment
          (bind _returnvalue_3 (Utilities|GetDataTableRow (Variables|Default|GetData%20Table) (Variables|Default|GetRow%20Name))
            (:then
              (Default|UpdateDialogue (Variables|Default|GetDialogueWidget) (.Dialogue (Utilities|Struct|BreakS_Dialogue _returnvalue_3)))
              (Variables|Default|SetRow%20Name (.Row (Utilities|Struct|BreakS_Dialogue _returnvalue_3)))
              (Variables|Default|SetData%20Table (.DataTable (Utilities|Struct|BreakS_Dialogue _returnvalue_3)))
              (Variables|Default|SetEndDialogue (.EndDialogue (Utilities|Struct|BreakS_Dialogue _returnvalue_3))))))
        (:Is%20Not%20Valid
          ;;[0.15 0.15 0.15 0.5] Comment
          (bind _returnvalue_4 (Utilities|GetDataTableRow (Variables|Default|GetData%20Table) (Variables|Default|GetRow%20Name))
            (:then
              (bind _returnvalue_5 (UserInterface|CreateWidget "/Game/UI/Widgets/WBP_Dialogue.WBP_Dialogue_C" 0 (Utilities|Text|ToText(Name) (Variables|Default|GetName)) (.Dialogue (Utilities|Struct|BreakS_Dialogue _returnvalue_4))))
              (bind _output_get (Variables|Default|SetDialogueWidget _returnvalue_5))
              (UserInterface|Viewport|AddtoViewport _output_get 0)
              (Variables|Default|SetRow%20Name (.Row (Utilities|Struct|BreakS_Dialogue _returnvalue_4)))
              (Variables|Default|SetData%20Table (.DataTable (Utilities|Struct|BreakS_Dialogue _returnvalue_4)))
              (Variables|Default|SetEndDialogue (.EndDialogue (Utilities|Struct|BreakS_Dialogue _returnvalue_4)))
              ;;[0.15 0.15 0.15 0.5] Comment
              (Input|SetInputModeGameandUI _returnvalue 0 "DoNotLock" true false)
              (Variables|/Script/Engine.PlayerController|SetbShowMouseCursor _returnvalue true)
              ;;[0.15 0.15 0.15 0.5] Comment
              (if (.OpenendedDialogue (Utilities|Struct|BreakS_Dialogue _returnvalue_4))
                (for _array_element (.OpenendedDialogueOptions (Utilities|Struct|BreakS_Dialogue _returnvalue_4))
                  (bind _returnvalue_6 (UserInterface|CreateWidget "/Game/UI/Widgets/WBP_Option.WBP_Option_C" 0 (Utilities|Text|ToText(Name) (.OptionName (Utilities|Struct|BreakS_OptionalDialogue _array_element))) self (.Row (Utilities|Struct|BreakS_OptionalDialogue _array_element)) (.DataTable (Utilities|Struct|BreakS_OptionalDialogue _array_element))))
                  (Widget|Panel|AddChild (Variables|/Game/UI/Widgets/WBP_Dialogue.WBP_Dialogue_C|GetScrollBox_1 (Variables|Default|GetDialogueWidget)) _returnvalue_6))))))))))