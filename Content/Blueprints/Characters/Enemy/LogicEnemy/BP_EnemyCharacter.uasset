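; Enemy character for a turn-based game that, on its turn, moves toward the player and then passes the turn on.
; BeginPlay caches the BP_TurnManager found in the level.
; EnemyTurn waits briefly for pacing, then runs AI MoveTo with the player's location and the passed target actor.
; Only a successful move calls EndEnemyTurn, which invokes NextTurn on the manager; PlayerRef is not assigned in these graphs.
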(event Custom|EnemyTurn
  (params (TargetActor :type Actor%20Object%20Reference))
  ;[0.6406 0 0 0.5] Oh shit:
  ; 1. A small delay (to visually create a sense of turn-based movement)
  ; 2. Movement toward the player via AI Move To
  ; 3. After completing the movement, call the EndEnemyTurn() event
  (Development|PrintString "Enemy Turn Started")
  (Utilities|FlowControl|Delay 0.5)
  ;;[0.000136 0.01157 0.15 0.5] The enemy gets the player's position and moves to it
  (AI|AIMoveTo self (Transformation|GetActorLocation (Variables|Default|GetPlayerRef)) TargetActor 1e+02 false
    (:OnSuccess
      (CallFunction|EndEnemyTurn))))

(event Custom|EndEnemyTurn
  ;[1 0.00036 0.03258 0.5] pass the move on
  (Default|NextTurn (Variables|Default|GetTurnManagerRef)))

(event EventBeginPlay
  ;[0.526 0 0 0.5] The enemy announces the end of his turn
  (bind _returnvalue (Actor|GetActorOfClass "/Game/Blueprints/Characters/Enemy/LogicEnemy/BP_TurnManager.BP_TurnManager_C"))
  (Variables|Default|SetTurnManagerRef _returnvalue))

(fn ConstructionScript)