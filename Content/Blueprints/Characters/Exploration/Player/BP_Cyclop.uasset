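; BP_Cyclop is the exploration player Blueprint that lets the player interact with nearby actors.
; A Sphere overlap caches the first component implementing BP_Interact on the overlapping actor as DialogueActor, and any end overlap clears it.
; Pressing the Enhanced Input action IA_Interact sends InteractMessage to that cached component, passing itself.
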(event OnComponentBeginOverlap(Sphere)
  (params (OverlappedComponent :type Primitive%20Component%20Object%20Reference) (OtherActor :type Actor%20Object%20Reference) (OtherComp :type Primitive%20Component%20Object%20Reference) (OtherBodyIndex :type Integer) (bFromSweep :type Boolean) (SweepResult :type Hit%20Result%20Structure%20%28by%20ref%29))
  ;[0.15 0.15 0.15 0.5] Comment
  (Variables|Default|SetDialogueActor (Utilities|Array|Get(acopy) (Class|Actor|GetComponentsbyInterface OtherActor "/Game/Blueprints/Dialogue/BP_Interact.BP_Interact_C"))))

(event OnComponentEndOverlap(Sphere)
  (params (OverlappedComponent :type Primitive%20Component%20Object%20Reference) (OtherActor :type Actor%20Object%20Reference) (OtherComp :type Primitive%20Component%20Object%20Reference) (OtherBodyIndex :type Integer))
  ;[0.15 0.15 0.15 0.5] Comment
  (Utilities|IsValid (Variables|Default|GetDialogueActor)
    (:Is%20Valid
      (Variables|Default|SetDialogueActor 0))))

(event Input|EnhancedActionEvents|EnhancedInputActionIA_Interact
  (params (ActionValue :type Boolean) (ElapsedSeconds :type Float%20%28double-precision%29) (TriggeredSeconds :type Float%20%28double-precision%29) (InputAction :type Input%20Action%20Object%20Reference :default "/Game/Input/Actions/IA_Interact.IA_Interact"))
  (bind _dialogueactor (Variables|Default|GetDialogueActor))
  ;[0.15 0.15 0.15 0.5] Comment
  (:Started
    (Utilities|IsValid _dialogueactor
      (:Is%20Valid
        (Class|BPInteract|Interact(Message) _dialogueactor self)))))

(fn ConstructionScript)