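; White Captivity character ability that applies a one-turn mind stun to an enemy on the tile grid.
; On start, it converts the cursor location to a tile and compares it with the tile of every BP_BaseEnemy, using a mixed X/Y equality test.
; When that test passes, it stuns the existing TargetActor rather than the looped enemy, then stops the ability.
; Debug strings in Russian trace each step.
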(fn StartAbility
  (bind _grid (Variables|Default|GetGrid))
  (|CallParentFunction)
  (Development|PrintString "способность активирована")
  (bind _location (Default|GetCursorLocationonGrid _grid))
  (bind _index (Default|GetTileIndexfromWorldLocation _grid _location))
  (bind _outactors (Actor|GetAllActorsOfClass (Variables|Default|GetOwningActor) "/Game/Blueprints/Characters/Tactical/Enemy/BP_BaseEnemy.BP_BaseEnemy_C"))
  (for _array_element _outactors
    (bind _index_2 (Default|GetTileIndexfromWorldLocation _grid (Transformation|GetActorLocation _array_element)))
    (Development|PrintString "переходим к с тану")
    (if (== (== (.x _index_2) (.y _index)) (== (.x _index) (.y _index_2)))
      (bind _targetactor (Variables|Default|GetTargetActor)
        (:then
          ;[0.15 0.15 0.15 0.5] накладывает стан
          (Utilities|Casting|CastToBP_BaseEnemy _targetactor)
          (Variables|Default|SetbIsCastingMindStun true)
          (Variables|Default|SetStunTurnsRemaining 1)
          (Development|PrintString "Враг в стане")
          (CallFunction|StopAbility))
        (:else)))))