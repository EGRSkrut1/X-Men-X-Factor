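; Base Blueprint for tactical units, providing the hook that ends a unit's turn.
; FinishMyTurn casts the game mode to BP_GameMode_Tactical and checks that CurrentTurn is in a specific state and that AttributeComponent places the unit in the player squad.
; When both hold, it prints a debug message and notifies the game mode through PlayerUnitFinished, using the unit's squad slot index.
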(fn ConstructionScript)

(fn FinishMyTurn
  (params (OutSlotIndex :type Integer))
  (bind _attributecomponent (Variables|Default|GetAttributeComponent))
  ;[0.15 0.15 0.15 0.5] Comment
  (bind _asbp_game_mode_tactical (Utilities|Casting|CastToBP_GameMode_Tactical (Game|GetGameMode)))
  (if (and (Utilities|Enum|Equal(Enum) (Variables|/Game/Blueprints/TacticalMode/BP_GameMode_Tactical.BP_GameMode_Tactical_C|GetCurrentTurn _asbp_game_mode_tactical) "NewEnumerator0") (Class|XAttributeComponent|IsinPlayerSquad _attributecomponent))
    (Development|PrintString "Finish unit turn")
    (Default|PlayerUnitFinished _asbp_game_mode_tactical OutSlotIndex)
    (return (Variables|/Script/Xmen_Xfactor.XAttributeComponent|GetSquadSlotIndex _attributecomponent))))