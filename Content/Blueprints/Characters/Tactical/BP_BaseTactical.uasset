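; Base tactical character for grid-based, turn-based combat that walks tile paths, performs basic attacks and reports finished turns.
; Path following uses a timeline scaled to per-tile duration, interpolating location and rotation, then recursing to the next tile.
; Left click plays the attack montage when ValidAttack passes its comparison of selected, target and non-diagonal neighbour tiles.
; The construction script finds BP_Grid, and FinishMyTurn notifies the tactical game mode for player-squad units.
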(event Custom|Event_FollowPath
  (params (Path :type Array%20of%20Int%20Point%20Structures))
  ;[0.15 0.15 0.15 0.5] Comment
  (if (> (Utilities|Array|Length Path) 0)
    (Variables|Default|SetCurrentPathToFollow Path)
    (CallFunction|ContinuetoFollowPath)))

(event Custom|ContinueToFollowPath
  (bind _timeline_unitmovement (Variables|Default|GetTimeline_UnitMovement))
  (bind _currentpathtofollow (Variables|Default|GetCurrentPathToFollow))
  (bind _grid (Variables|Default|GetGrid))
  (bind _output (Utilities|Array|Get(acopy) _currentpathtofollow))
  (bind _gridtiles (Variables|/Game/Blueprints/TacticalMode/Bp_Grid.BP_Grid_C|GetGridTiles _grid))
  (bind _value (Utilities|Map|Find _gridtiles _output))
  (bind _transform (Utilities|Struct|BreakS_TileData _value))
  ;[0.15 0.15 0.15 0.5] Comment
  (if (> (Utilities|Array|Length (Variables|Default|GetCurrentPathToFollow)) 0)
    (Variables|Default|SetPreviousTransform (Transformation|GetActorTransform))
    (Variables|Default|SetNextTransform (Math|Transform|MakeTransform (.location _transform) (Math|Rotator|FindLookatRotation (.location (Variables|Default|GetPreviousTransform)) (.location _transform)) "1.000000,1.000000,1.000000"))
    (Components|Timeline|SetPlayRate _timeline_unitmovement (/ (Components|Timeline|GetTimelineLength _timeline_unitmovement) (Variables|Default|GetMoveDurationPerTile)))
    (bind (_direction _locationalpha _rotationalpha) (Timeline|Timeline_UnitMovement PlayFromStart)
      (:Update
        (Transformation|SetActorLocationAndRotation (Math|Vector|Lerp(Vector) (.location (Variables|Default|GetPreviousTransform)) (Math|Vector|MakeVector (.x (.location (Variables|Default|GetNextTransform))) (.y (.location (Variables|Default|GetNextTransform))) (+ (.z (.location (Variables|Default|GetNextTransform))) (Components|Capsule|GetScaledCapsuleHalfHeight (Variables|Default|GetCapsuleComponent)))) _locationalpha) (Math|Rotator|MakeRotator (.roll (Math|Rotator|Lerp(Rotator) (.rotation (Variables|Default|GetPreviousTransform)) (.rotation (Variables|Default|GetNextTransform)) _rotationalpha true)) 0.0 (.yaw (Math|Rotator|Lerp(Rotator) (.rotation (Variables|Default|GetPreviousTransform)) (.rotation (Variables|Default|GetNextTransform)) _rotationalpha true)))))
      (:Finished
        (Utilities|Array|RemoveIndex (Variables|Default|GetCurrentPathToFollow))
        (CallFunction|ContinuetoFollowPath)))))

(event Input|MouseEvents|LeftMouseButton
  (params (Key :type Key%20Structure))
  ;[0.15 0.15 0.15 0.5] Comment
  (:Pressed
    (bind _canattack (CallFunction|ValidAttack))
    (if _canattack
      (CallFunction|PlayMontageAttack)
      (else
        (Development|PrintString "Can't attack")))))

(fn ConstructionScript
  (bind _returnvalue (Actor|GetActorOfClass "/Game/Blueprints/TacticalMode/Bp_Grid.BP_Grid_C"))
  (Variables|Default|SetGrid _returnvalue))

(fn ValidAttack
  (params (target%20actor :type BP%20Base%20Tactical%20Object%20Reference))
  (bind _playergridactions (Variables|Default|GetPlayerGridActions))
  (bind _playergridactions_2 (Variables|Default|GetPlayerGridActions))
  (bind _grid (Variables|Default|GetGrid))
  (bind _selectedtile (Variables|/Game/Blueprints/TacticalMode/BP_PlayerGridActions.BP_PlayerGridActions_C|GetSelectedTile _playergridactions))
  (bind _selectedtile_2 (Variables|/Game/Blueprints/TacticalMode/BP_PlayerGridActions.BP_PlayerGridActions_C|GetSelectedTile _playergridactions_2))
  ;[0.15 0.15 0.15 0.5] is the enemy on the cage
  (bind _index (Default|GetTileIndexfromWorldLocation (Variables|Default|GetGrid) (Transformation|GetActorLocation target%20actor)))
  ;[0.15 0.15 0.15 0.5] Is the selected cell in the neighboring cells
  (bind _index_2 (Default|GetTileIndexfromWorldLocation _grid (Transformation|GetActorLocation)))
  (bind _neighbours (Default|GetNeighboursIndexes (Variables|/Game/Blueprints/TacticalMode/Bp_Grid.BP_Grid_C|GetGridPathfinding _grid) _index_2 false))
  (for _array_element _neighbours
    ;[0.15 0.15 0.15 0.5] Comment
    (if (== (== (== (.x _selectedtile_2) (.x _index)) (== (.y _selectedtile_2) (.y _index))) (== (== (.x _selectedtile) (.X (Utilities|Struct|BreakIntPoint _array_element))) (== (.y _selectedtile) (.Y (Utilities|Struct|BreakIntPoint _array_element)))))
      (return true)))
  (return false))

(fn PlayMontageAttack
  ;[0.15 0.15 0.15 0.5] Comment
  (Animation|Montage|MontagePlay (Components|SkeletalMesh|GetAnimInstance (Variables|Character|GetMesh)) "/Game/Animation/Characters/Unarmed/AM_BasicAttack.AM_BasicAttack" 1.0 "MontageLength" 0.0 true))

(fn SetGrid
  (params (Grid :type BP%20Grid%20Object%20Reference))
  (Variables|Default|SetGrid Grid))

(fn FinishMyTurn
  (params (OutSlotIndex :type Integer))
  (bind _attributecomponent (Variables|Default|GetAttributeComponent))
  ;[0.15 0.15 0.15 0.5] Comment
  (bind _asbp_game_mode_tactical (Utilities|Casting|CastToBP_GameMode_Tactical (Game|GetGameMode)))
  (if (and (Utilities|Enum|Equal(Enum) (Variables|/Game/Blueprints/TacticalMode/BP_GameMode_Tactical.BP_GameMode_Tactical_C|GetCurrentTurn _asbp_game_mode_tactical) "NewEnumerator0") (Class|XAttributeComponent|IsinPlayerSquad _attributecomponent))
    (Development|PrintString "Finish unit turn")
    (Default|PlayerUnitFinished _asbp_game_mode_tactical OutSlotIndex)
    (return (Variables|/Script/Xmen_Xfactor.XAttributeComponent|GetSquadSlotIndex _attributecomponent))))